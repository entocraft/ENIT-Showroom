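; A detection zone actor that shows the info menu while the XR pawn is inside its box volume.
; When a BP_XRPawn begins overlapping the Box, it finds the BP_InfoMenu in the level, makes its Menu component and children visible, and enables that actor's collision.
; When the pawn leaves, it hides the menu and disables its collision.
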(event OnComponentBeginOverlap(Box)
  (params (OverlappedComponent :type Primitive%20Component%20Object%20Reference) (OtherActor :type Actor%20Object%20Reference) (OtherComp :type Primitive%20Component%20Object%20Reference) (OtherBodyIndex :type Integer) (bFromSweep :type Boolean) (SweepResult :type Hit%20Result%20Structure%20%28by%20ref%29))
  (Utilities|Casting|CastToBP_XRPawn OtherActor)
  (bind _returnvalue (Actor|GetActorOfClass "/Game/Assets/Objects/BP_InfoMenu.BP_InfoMenu_C"))
  (Rendering|SetVisibility (Variables|/Game/Assets/Objects/BP_InfoMenu.BP_InfoMenu_C|GetMenu _returnvalue) true true)
  (Collision|SetActorEnableCollision _returnvalue true))

(event OnComponentEndOverlap(Box)
  (params (OverlappedComponent :type Primitive%20Component%20Object%20Reference) (OtherActor :type Actor%20Object%20Reference) (OtherComp :type Primitive%20Component%20Object%20Reference) (OtherBodyIndex :type Integer))
  (Utilities|Casting|CastToBP_XRPawn OtherActor)
  (bind _returnvalue (Actor|GetActorOfClass "/Game/Assets/Objects/BP_InfoMenu.BP_InfoMenu_C"))
  (Rendering|SetVisibility (Variables|/Game/Assets/Objects/BP_InfoMenu.BP_InfoMenu_C|GetMenu _returnvalue) false true)
  (Collision|SetActorEnableCollision _returnvalue false))

(event EventBeginPlay)

(event Collision|EventActorBeginOverlap
  (params (OtherActor :type Actor%20Object%20Reference)))

(event EventTick
  (params (DeltaSeconds :type Float%20%28single-precision%29)))

(fn ConstructionScript)