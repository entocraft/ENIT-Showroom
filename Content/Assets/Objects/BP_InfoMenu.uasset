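; BP_InfoMenu is a VR info menu actor whose Menu component and its children start hidden at BeginPlay.
; SetMotionControllerReference searches the player pawn's motion controllers and caches the left or right aim controller, chosen by the active menu hand.
; It prints a warning when the pawn has no motion controllers, though the message names a missing WidgetInteractionComponent.
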(event EventBeginPlay
  (Rendering|SetVisibility (Variables|Components|GetMenu) false true))

(event Collision|EventActorBeginOverlap
  (params (OtherActor :type Actor%20Object%20Reference)))

(event EventTick
  (params (DeltaSeconds :type Float%20%28single-precision%29)))

(fn ConstructionScript)

(fn SetMotionControllerReference
  (bind _returnvalue (Game|Player|GetPlayerPawn 0))
  (bind _returnvalue_2 (Actor|GetComponentsByClass _returnvalue "/Script/HeadMountedDisplay.MotionControllerComponent"))
  (if (> (Utilities|Array|Length _returnvalue_2) 0) ; Are there any Motion Controllers attached to the Player Pawn?
    (bind _output_get (LocalVariables|SetLocalMotionControllers _returnvalue_2))
    (for _array_element _output_get
      (if (Utilities|Name|Equal(Name) (Variables|/Script/HeadMountedDisplay.MotionControllerComponent|GetMotionSource _array_element) (select (Variables|Components|GetbActiveMenuHandRight) "RightAim" "LeftAim"))
        (Variables|Components|SetMotionControllerAimRef _array_element)))
    (else
      (Development|PrintString "Warning: No WidgetInteractionComponent was found. Menu interaction will FAIL"))))