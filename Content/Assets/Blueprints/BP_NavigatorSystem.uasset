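; BP_NavigatorSystem shows a navigation route from the XR pawn's navigator point to the PointB actor.
; RecalcPath runs a synchronous navmesh path query, flushes old debug lines and draws the path segments as long-lived green debug lines.
; Tick triggers a recalculation whenever the navigator point moves beyond a small distance from its last recorded position.
; BeginPlay also starts a looping timer, whose bound event is unspecified.
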(event Custom|RecalcPath
  (Rendering|Debug|FlushPersistentDebugLines)
  (bind _asbp_xrpawn (Utilities|Casting|CastToBP_XRPawn (Game|Player|GetPlayerPawn 0)))
  (bind _returnvalue (Class|NavigationSystemV1|FindPathtoLocationSynchronously (Transformation|GetWorldLocation (Variables|/Game/XRFramework/Blueprints/BP_XRPawn.BP_XRPawn_C|GetBP_NavigatorPoint _asbp_xrpawn)) (Transformation|GetActorLocation (Variables|Default|GetPointB)) 0 0))
  (for (_array_element _array_index) (Variables|/Script/NavigationSystem.NavigationPath|GetPathPoints _returnvalue)
    (if (< (+ _array_index 1) (Utilities|Array|Length (Variables|/Script/NavigationSystem.NavigationPath|GetPathPoints _returnvalue)))
      (Rendering|Debug|DrawDebugLine _array_element (Utilities|Array|Get(acopy) (Variables|/Script/NavigationSystem.NavigationPath|GetPathPoints _returnvalue) (+ _array_index 1)) "(R=0.000000,G=1.000000,B=0.313357,A=1.000000)" 9999.0 5.0))))

(event EventBeginPlay
  (Utilities|Time|SetTimerbyEvent (EventDispatchers|CreateEvent :!event Custom|RecalcPath) 1.0 true))

(event EventTick
  (params (DeltaSeconds :type Float%20%28single-precision%29))
  (bind _asbp_xrpawn (Utilities|Casting|CastToBP_XRPawn (Game|Player|GetPlayerPawn 0)))
  (if (> (Math|Vector|Distance(Vector) (Transformation|GetWorldLocation (Variables|/Game/XRFramework/Blueprints/BP_XRPawn.BP_XRPawn_C|GetBP_NavigatorPoint _asbp_xrpawn)) (Variables|Default|GetLastPos)) 2e+01)
    (CallFunction|RecalcPath)
    (Variables|Default|SetLastPos (Transformation|GetWorldLocation (Variables|/Game/XRFramework/Blueprints/BP_XRPawn.BP_XRPawn_C|GetBP_NavigatorPoint _asbp_xrpawn)))))

(fn ConstructionScript)